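; Player-controlled P-38 plane that flies continuously forward and fires rockets.
; Tick feeds the forward vector scaled by Speed into movement input, which the Boost action raises while held.
; Lookup and LookRight axes apply frame-rate-independent local pitch and roll, while BeginPlay registers both propeller meshes with the BPPropellerRotation component.
; FireMisslie spawns a BP_Rocket just below the plane and attaches a particle emitter to its mesh.
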(event EventBeginPlay
  (Utilities|Array|Add (Variables|/Game/Blueprints/BP_PropellerRotation.BP_PropellerRotation_C|GetSceneComponentRight (Variables|Default|GetBP_PropellerRotation)) (Variables|Default|GetSM_P38_Propeller_Right))
  (Utilities|Array|Add (Variables|/Game/Blueprints/BP_PropellerRotation.BP_PropellerRotation_C|GetSceneComponentLeft (Variables|Default|GetBP_PropellerRotation)) (Variables|Default|GetSM_P38_Propeller_Left)))

(event Collision|EventActorBeginOverlap
  (params (OtherActor :type Actor%20Object%20Reference)))

(event EventTick
  (params (DeltaSeconds :type Float%20%28single-precision%29))
  (Pawn|Input|AddMovementInput (* (Transformation|GetActorForwardVector) (Variables|Default|GetSpeed)) 1.0 false))

(event Input|ActionEvents|InputActionBoost
  (params (Key :type Key%20Structure :default "None"))
  (:Pressed
    (Variables|Default|SetSpeed 1.0))
  (:Released
    (Variables|Default|SetSpeed 0.5)))

(event Input|ActionEvents|InputActionFireMisslie
  (params (Key :type Key%20Structure :default "None"))
  (bind _returnvalue (Transformation|GetActorTransform))
  (:Pressed
    (bind _returnvalue_2 (Game|SpawnActorfromClass "/Game/Blueprints/BP_Rocket.BP_Rocket_C" (Math|Transform|MakeTransform (Math|Vector|MakeVector (.x (.location _returnvalue)) (.y (.location _returnvalue)) (+ (.z (.location _returnvalue)) -25.0)) (.rotation _returnvalue) (.scale _returnvalue)) "AlwaysSpawn" "MultiplyWithRoot" 0 0))
    (bind _asbp_rocket (Utilities|Casting|CastToBP_Rocket _returnvalue_2))
    (Effects|SpawnEmitterAttached "/Engine/Tutorial/SubEditors/TutorialAssets/TutorialParticleSystem.TutorialParticleSystem" (Variables|/Game/Blueprints/BP_Rocket.BP_Rocket_C|GetStaticMesh _asbp_rocket) "None" "0, 0, 0" "0, 0, 0" "0.200000,0.200000,0.200000")))

(event Input|AxisEvents|InputAxisLookup
  (params (AxisValue :type Float%20%28single-precision%29))
  (Transformation|AddActorLocalRotation (Math|Rotator|MakeRotator 0.0 (* AxisValue (Variables|Default|GetRotateSpeed) (Utilities|Time|GetWorldDeltaSeconds)) 0.0) false false))

(event Input|AxisEvents|InputAxisLookRight
  (params (AxisValue :type Float%20%28single-precision%29))
  (Transformation|AddActorLocalRotation (Math|Rotator|MakeRotator (* AxisValue (Variables|Default|GetRotateSpeed) (Utilities|Time|GetWorldDeltaSeconds)) 0.0 0.0) false false))

(fn ConstructionScript)