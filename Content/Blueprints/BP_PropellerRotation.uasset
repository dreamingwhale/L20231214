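; Propeller rotation Blueprint that spins left and right sets of scene components in opposite roll directions.
; Each Tick, Speed compounds by a DeltaSeconds-scaled fraction of itself while the result stays within MaxSpeed, giving an exponential spin-up from its starting value.
; Speed is then applied as a per-frame local roll, positive for the left array and negative for the right, so rotation rate depends on framerate.
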(event EventBeginPlay)

(event EventTick
  (params (DeltaSeconds :type Float%20%28single-precision%29))
  (Utilities|FlowControl|Sequence
    (:then_0
      (if (<= (+ (* DeltaSeconds (Variables|Default|GetSpeed)) (Variables|Default|GetSpeed)) (Variables|Default|GetMaxSpeed))
        (Variables|Default|SetSpeed (+ (* DeltaSeconds (Variables|Default|GetSpeed)) (Variables|Default|GetSpeed)))))
    (:then_1
      (for _array_element (Variables|Default|GetSceneComponentLeft)
        (Transformation|AddLocalRotation _array_element (Math|Rotator|MakeRotator (* (Variables|Default|GetSpeed) 1.0) 0.0 0.0) false false)))
    (:then_2
      (for _array_element_2 (Variables|Default|GetSceneComponentRight)
        (Transformation|AddLocalRotation _array_element_2 (Math|Rotator|MakeRotator (* (Variables|Default|GetSpeed) -1.0) 0.0 0.0) false false)))))